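; BP_Door is an interactable door actor that swings open or closed on its yaw axis.
; Interact plays a door sound and restarts the DoorOpen timeline, whose DoorRotation track drives the Door component's relative rotation.
; IsOpen selects between the raw track value and one offset by 90 degrees to reverse the swing.
; The flag flips through a one-second Delay chained to the timeline's Update rather than Finished.
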(event EventBeginPlay)

(event Collision|EventActorBeginOverlap
  (params (OtherActor :type Actor%20Object%20Reference)))

(event EventTick
  (params (DeltaSeconds :type Float%20%28single-precision%29)))

(event EventInteract
  (Audio|Components|Audio|Play (Variables|Default|Get15419__pagancow__dorm-door-opening_Cue) 0.5)
  (bind _doorrotation (Timeline|DoorOpen PlayFromStart)
    (:Update
      (if (Variables|Default|GetisOpen)
        ;[1 1 1] Door Open
        (bind _result (Math|Float|NegateFloat (- _doorrotation 9e+01))
          (:%20%20
            (Transformation|SetRelativeRotation (Variables|Default|GetDoor) (Math|Rotator|MakeRotator 0.0 0.0 _result) false false)))
        (else
          ;[1 1 1] Door Close
          (Transformation|SetRelativeRotation (Variables|Default|GetDoor) (Math|Rotator|MakeRotator 0.0 0.0 _doorrotation) false false)))
      (Utilities|FlowControl|Delay 1.0)
      (CallFunction|ToggleDoorRotation))))

(fn ConstructionScript)

(fn ToggleDoorRotation
  (if (Variables|Default|GetisOpen)
    (Variables|Default|SetisOpen false)
    (else
      (Variables|Default|SetisOpen true))))