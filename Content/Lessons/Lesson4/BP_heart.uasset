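; BP_heart is a lesson actor that toggles a vertical bobbing motion each time its SwitchInteraction event fires.
; Switching on stores the current location as Origin, waits a short random delay, then plays the UpAndDown timeline to offset the actor along Z from that origin.
; Switching off returns the actor to Origin and stops the timeline, though it does not cancel a pending delay.
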(event EventBeginPlay)

(event Collision|EventActorBeginOverlap
  (params (OtherActor :type Actor%20Object%20Reference)))

(event EventSwitchInteraction
  (CallFunction|ToggleTimeline)
  (if (Variables|Default|GetisOn)
    (bind _output_get (Variables|Default|SetOrigin (Transformation|GetActorLocation)))
    (Utilities|FlowControl|Delay (Math|Random|RandomFloatinRange 0.0 2.0))
    (bind _data (Timeline|UpAndDown PlayFromStart)
      (:Update
        (Transformation|SetActorLocation (+ (* "0.0,0.0,5.000000" _data) (Variables|Default|GetOrigin)) false false)))
    (else
      (Transformation|SetActorLocation _output_get false false)
      (Timeline|UpAndDown Stop))))

(event EventTick
  (params (DeltaSeconds :type Float%20%28single-precision%29)))

(fn ConstructionScript)

(fn ToggleTimeline
  (if (Variables|Default|GetisOn)
    (Variables|Default|SetisOn false)
    (else
      (Variables|Default|SetisOn true))))