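; BP_HW4Players is a first-person player pawn with movement, look controls, a gaze reticle and click-to-interact.
; Each tick, a visibility trace along the VR camera's forward vector places a MaterialBillboard reticle at the hit point, or at the trace end on a miss.
; Left mouse click repeats the trace and calls InteractMessage on the hit actor.
; Axis inputs drive movement along actor forward and right vectors, plus controller yaw and pitch.
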(event EventBeginPlay)

(event Collision|EventActorBeginOverlap
  (params (OtherActor :type Actor%20Object%20Reference)))

(event EventTick
  (params (DeltaSeconds :type Float%20%28single-precision%29))
  ;[1 1 1] Reticle
  (bind (_location _forward_vector) (CallFunction|GetPlayerVRCameraProperties))
  (bind (_outhit _returnvalue) (Collision|LineTraceByChannel _location (+ (* _forward_vector 1e+04) _location) "TraceTypeQuery1" false 0 "None"))
  (if _returnvalue
    (Transformation|SetWorldLocation (Variables|Default|GetMaterialBillboard) (.Location (Collision|BreakHitResult _outhit)) false false)
    (else
      (Transformation|SetWorldLocation (Variables|Default|GetMaterialBillboard) (+ (* _forward_vector 1e+04) _location) false false))))

(event Input|AxisEvents|InputAxisMoveForward
  (params (AxisValue :type Float%20%28single-precision%29))
  (Pawn|Input|AddMovementInput (Transformation|GetActorForwardVector) AxisValue false))

(event Input|AxisEvents|InputAxisLookUp
  (params (AxisValue :type Float%20%28single-precision%29))
  (Pawn|Input|AddControllerPitchInput AxisValue))

(event Input|AxisEvents|InputAxisMoveRight
  (params (AxisValue :type Float%20%28single-precision%29))
  (Pawn|Input|AddMovementInput (Transformation|GetActorRightVector) AxisValue false))

(event Input|AxisEvents|InputAxisTurn
  (params (AxisValue :type Float%20%28single-precision%29))
  (Pawn|Input|AddControllerYawInput AxisValue))

(event Input|MouseEvents|LeftMouseButton
  (params (Key :type Key%20Structure :default "AnyKey"))
  ;[1 1 1] Object Interaction on click
  (:Pressed
    (bind (_location _forward_vector) (CallFunction|GetPlayerVRCameraProperties))
    (bind (_outhit _returnvalue) (Collision|LineTraceByChannel _location (+ (* _forward_vector 1e+04) _location) "TraceTypeQuery1" false 0 "None"))
    (if _returnvalue
      (Class|BPIHW4Interaction|Interact(Message) (.HitActor (Collision|BreakHitResult _outhit))))))

(fn ConstructionScript)