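; Lesson 3 player Blueprint that lets the user aim at and interact with actors by looking at them through the VR camera.
; BeginPlay calls AddBPCCameraControl to set up camera control.
; Every Tick, a long Visibility trace along the camera's forward vector moves a MaterialBillboard reticle to the hit point, or the ray's end.
; Pressing Act repeats the trace and sends InteractMessage to the hit actor.
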(event EventBeginPlay
  (AddComponent|AddBPCCameraControl))

(event Collision|EventActorBeginOverlap
  (params (OtherActor :type Actor%20Object%20Reference)))

(event EventTick
  (params (DeltaSeconds :type Float%20%28single-precision%29))
  (bind (_location _forward_vector) (CallFunction|GetPlayerVRCameraProperties))
  (bind (_outhit _returnvalue) (Collision|LineTraceByChannel _location (+ _location (* _forward_vector 100000)) "TraceTypeQuery1" false 0 "None"))
  (if _returnvalue
    (Transformation|SetWorldLocation (Variables|Default|GetMaterialBillboard) (.Location (Collision|BreakHitResult _outhit)) false false)
    (else
      (Transformation|SetWorldLocation (Variables|Default|GetMaterialBillboard) (+ _location (* _forward_vector 100000)) false false))))

(event Input|ActionEvents|InputActionAct
  (params (Key :type Key%20Structure :default "AnyKey"))
  (:Pressed
    (bind (_location _forward_vector) (CallFunction|GetPlayerVRCameraProperties))
    (bind (_outhit _returnvalue) (Collision|LineTraceByChannel _location (+ _location (* _forward_vector 100000)) "TraceTypeQuery1" false 0 "None" true "(R=1.000000,G=0.000000,B=0.000000,A=1.000000)" "(R=0.000000,G=1.000000,B=0.000000,A=1.000000)" 1.0))
    (if _returnvalue
      (Class|BPIInteraction|Interact(Message) (.HitActor (Collision|BreakHitResult _outhit))))))

(fn ConstructionScript)